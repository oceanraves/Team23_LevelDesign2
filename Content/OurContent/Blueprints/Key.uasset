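; Key pickup that removes a door obstacle from the level when something overlaps it.
; A Hover timeline started on BeginPlay eases the cylinder toward MaxPos and steadily increments the root's yaw to spin it.
; The box collider's first overlap, with no effective filter on the other actor, destroys the Door_Obstacle found by GetActorOfClass, then the key itself.
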(event `self.ReceiveBeginPlay`
  (bind (_direction _newtrack_0) (`Timeline|Hover`)
    (:`Update`
      (`SceneComponent.K2_SetRelativeLocation` (`self.Cylinder`) (`|EaseFunction` "Linear" _newtrack_0 (0.0 0.0 0.0) (`self.MaxPos`)) false false)
      (bind _output_get (set `self.zRot` (+ (`self.zRot`) 0.4)))
      (`SceneComponent.K2_SetWorldRotation` (`self.DefaultSceneRoot`) (`KismetMathLibrary.MakeRotator` 0.0 0.0 _output_get) false false))))

(event `self.BoxCollider.OnComponentBeginOverlap`
  (params (OverlappedComponent :type "PrimitiveComponent Object Reference") (OtherActor :type "Actor Object Reference") (OtherComp :type "PrimitiveComponent Object Reference") (OtherBodyIndex :type Integer) (bFromSweep :type Boolean) (SweepResult :type "HitResult Structure (by ref)"))
  (`GameplayStatics.GetActorOfClass` (`GameplayStatics.GetObjectClass` OtherActor))
  (`/Engine/EditorBlueprintResources/StandardMacros.DoOnce` false
    (:`Completed`
      (bind _returnvalue (`GameplayStatics.GetActorOfClass` "/Game/OurContent/Blueprints/Door_Obstacle.Door_Obstacle_C"))
      (`self.K2_DestroyActor` _returnvalue)
      (`self.K2_DestroyActor`))))

(fn `UserConstructionScript`)